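; InventoryComponent is an inventory component that holds a saved health pickup value and can add health to the player character.
; On BeginPlay it restores HealthPickup from the SaveGameData in MyGameInstance and caches player 0's ThirdPersonCharacter.
; AddHealth re-fetches that character and raises CurrHealth by AddHealthNumber, without clamping or changing HealthPickup.
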(event EventBeginPlay
  (bind _asmy_game_instance (Utilities|Casting|CastToMyGameInstance (Game|GetGameInstance)))
  (Variables|Default|SetHealthPickup (Variables|/Game/Blueprints/Saving/SaveGameObject.SaveGameObject_C|GetSavedHealthPickup (Variables|/Game/Blueprints/Saving/MyGameInstance.MyGameInstance_C|GetSaveGameData _asmy_game_instance)))
  (bind _asthird_person_character (Utilities|Casting|CastToThirdPersonCharacter (Game|GetPlayerCharacter 0)))
  (Variables|Default|SetPlayer _asthird_person_character))

(fn AddHealth
  (bind _asthird_person_character (Utilities|Casting|CastToThirdPersonCharacter (Game|GetPlayerCharacter 0)))
  (Variables|/Game/Blueprints/ThirdPersonCharacter.ThirdPersonCharacter_C|SetcurrHealth _asthird_person_character (+ (Variables|/Game/Blueprints/ThirdPersonCharacter.ThirdPersonCharacter_C|GetcurrHealth _asthird_person_character) (Variables|Default|GetAddHealthNumber))))