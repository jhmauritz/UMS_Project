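; LoadLevel is a trigger actor that teleports the player from a station hub to the level selected there.
; On BeginPlay it caches the StationPLayerHub actor found in the world.
; When the player pawn overlaps its Box, a Sequence checks each of the hub's region/station pressed flags.
; Each set flag sets IsTeleporting, waits a configurable delay, then opens the matching R#_S# level by name.
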(event OnComponentBeginOverlap(Box)
  (params (OverlappedComponent :type Primitive%20Component%20Object%20Reference) (OtherActor :type Actor%20Object%20Reference) (OtherComp :type Primitive%20Component%20Object%20Reference) (OtherBodyIndex :type Integer) (bFromSweep :type Boolean) (SweepResult :type Hit%20Result%20Structure%20%28by%20ref%29))
  (bind _stationref (Variables|Default|GetStationRef))
  (bind _durationdelay (Variables|Default|GetDurationDelay))
  (if (== OtherActor (Game|Player|GetPlayerPawn 0))
    (Utilities|FlowControl|Sequence
      (:then_0
        (if (Variables|/Game/Blueprints/StationPLayerHub.StationPLayerHub_C|GetR1_S1_Pressed _stationref)
          (Variables|Default|SetIsTeleporting true)
          (Utilities|FlowControl|Delay _durationdelay)
          (Game|OpenLevel(byName) "R1_S1")))
      (:then_1
        (if (Variables|/Game/Blueprints/StationPLayerHub.StationPLayerHub_C|GetR1_S2_Pressed _stationref)
          (Variables|Default|SetIsTeleporting true)
          (Utilities|FlowControl|Delay _durationdelay)
          (Game|OpenLevel(byName) "R1_S2")))
      (:then_2
        (if (Variables|/Game/Blueprints/StationPLayerHub.StationPLayerHub_C|GetR2_S1_Pressed _stationref)
          (Variables|Default|SetIsTeleporting true)
          (Utilities|FlowControl|Delay _durationdelay)
          (Game|OpenLevel(byName) "R2_S1")))
      (:then_3
        (if (Variables|/Game/Blueprints/StationPLayerHub.StationPLayerHub_C|GetR2_S2_Pressed _stationref)
          (Variables|Default|SetIsTeleporting true)
          (Utilities|FlowControl|Delay _durationdelay)
          (Game|OpenLevel(byName) "R2_S2")))
      (:then_4
        (if (Variables|/Game/Blueprints/StationPLayerHub.StationPLayerHub_C|GetR2_S3_Pressed _stationref)
          (Variables|Default|SetIsTeleporting true)
          (Utilities|FlowControl|Delay _durationdelay)
          (Game|OpenLevel(byName) "R2_S3")))
      (:then_5
        (if (Variables|/Game/Blueprints/StationPLayerHub.StationPLayerHub_C|GetR3_S1_Pressed _stationref)
          (Variables|Default|SetIsTeleporting true)
          (Utilities|FlowControl|Delay _durationdelay)
          (Game|OpenLevel(byName) "R3_S1")))
      (:then_6
        (if (Variables|/Game/Blueprints/StationPLayerHub.StationPLayerHub_C|GetR3_S2_Pressed _stationref)
          (Variables|Default|SetIsTeleporting true)
          (Utilities|FlowControl|Delay _durationdelay)
          (Game|OpenLevel(byName) "R3_S2")))
      (:then_7
        (if (Variables|/Game/Blueprints/StationPLayerHub.StationPLayerHub_C|GetR3_S3_Pressed _stationref)
          (Variables|Default|SetIsTeleporting true)
          (Utilities|FlowControl|Delay _durationdelay)
          (Game|OpenLevel(byName) "R3_S3")))
      (:then_8
        (if (Variables|/Game/Blueprints/StationPLayerHub.StationPLayerHub_C|GetR3_S4_Pressed _stationref)
          (Variables|Default|SetIsTeleporting true)
          (Utilities|FlowControl|Delay _durationdelay)
          (Game|OpenLevel(byName) "R3_S4")))
      (:then_9
        (if (Variables|/Game/Blueprints/StationPLayerHub.StationPLayerHub_C|GetR4_S1_Pressed _stationref)
          (Variables|Default|SetIsTeleporting true)
          (Utilities|FlowControl|Delay _durationdelay)
          (Game|OpenLevel(byName) "R4_S1")))
      (:then_10
        (if (Variables|/Game/Blueprints/StationPLayerHub.StationPLayerHub_C|GetR4_S2_Pressed _stationref)
          (Variables|Default|SetIsTeleporting true)
          (Utilities|FlowControl|Delay _durationdelay)
          (Game|OpenLevel(byName) "R4_S2")))
      (:then_11
        (if (Variables|/Game/Blueprints/StationPLayerHub.StationPLayerHub_C|GetR4_S3_Pressed _stationref)
          (Variables|Default|SetIsTeleporting true)
          (Utilities|FlowControl|Delay _durationdelay)
          (Game|OpenLevel(byName) "R4_S3")))
      (:then_12
        (if (Variables|/Game/Blueprints/StationPLayerHub.StationPLayerHub_C|GetR5_S1_Pressed _stationref)
          (Variables|Default|SetIsTeleporting true)
          (Utilities|FlowControl|Delay _durationdelay)
          (Game|OpenLevel(byName) "R5_S1")))
      (:then_13
        (if (Variables|/Game/Blueprints/StationPLayerHub.StationPLayerHub_C|GetR5_S2_Pressed _stationref)
          (Variables|Default|SetIsTeleporting true)
          (Utilities|FlowControl|Delay _durationdelay)
          (Game|OpenLevel(byName) "R5_S2"))))))

(event EventBeginPlay
  (bind _returnvalue (Actor|GetActorOfClass "/Game/Blueprints/StationPLayerHub.StationPLayerHub_C"))
  (Variables|Default|SetStationRef _returnvalue))

(event Collision|EventActorBeginOverlap
  (params (OtherActor :type Actor%20Object%20Reference)))

(event EventTick
  (params (DeltaSeconds :type Float%20%28single-precision%29)))

(fn ConstructionScript)