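; Game instance that owns the game and options save objects for the session.
; On Init it loads each save from its slot, or creates and writes a new one if none exists.
; Save and load functions copy the player's position between the third-person character and the save object, moving the actor on load; saving does not write to disk.
; The options save and load functions are unfinished stubs.
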(event EventInit
  (Utilities|FlowControl|Sequence
    (:then_0
      (CallFunction|OptionsSaveHandler))
    (:then_1
      (CallFunction|GameSaveHandler))))

(fn SavePlayerData
  (bind _asthird_person_character (Utilities|Casting|CastToThirdPersonCharacter (Game|GetPlayerCharacter 0)))
  (bind _output_get (LocalVariables|SetPlayerRef _asthird_person_character))
  (Variables|/Game/Blueprints/Saving/SaveGameObject.SaveGameObject_C|SetplayerPos (Variables|Default|GetSaveGameData) (Variables|/Game/Blueprints/ThirdPersonCharacter.ThirdPersonCharacter_C|GetplayerPosition _output_get)))

(fn LoadPlayerData
  (bind _asthird_person_character (Utilities|Casting|CastToThirdPersonCharacter (Game|GetPlayerCharacter 0)))
  (bind _output_get (LocalVariables|SetPlayerRef _asthird_person_character))
  (bind _output_get_2 (Variables|/Game/Blueprints/ThirdPersonCharacter.ThirdPersonCharacter_C|SetplayerPosition _output_get (Variables|/Game/Blueprints/Saving/SaveGameObject.SaveGameObject_C|GetplayerPos (Variables|Default|GetSaveGameData))))
  (Transformation|SetActorLocation (LocalVariables|GetPlayerRef) _output_get_2 false false))

(fn OptionsSaveHandler
  (bind _returnvalue (SaveGame|DoesSaveGameExist (Variables|Default|GetOptionsSlotName)))
  (if _returnvalue
    (bind _returnvalue_2 (SaveGame|LoadGamefromSlot (Variables|Default|GetOptionsSlotName)))
    (bind _asoptions_save (Utilities|Casting|CastToOptionsSave _returnvalue_2))
    (Variables|Default|SetOptionsSave _asoptions_save)
    (else
      (bind _returnvalue_3 (SaveGame|CreateSaveGameObject "/Game/Blueprints/Saving/OptionsSave.OptionsSave_C"))
      (bind _output_get (Variables|Default|SetOptionsSave _returnvalue_3))
      (SaveGame|SaveGametoSlot _output_get (Variables|Default|GetOptionsSlotName)))))

(fn GameSaveHandler
  (bind _returnvalue (SaveGame|DoesSaveGameExist (Variables|Default|GetSaveSlotName)))
  (if _returnvalue
    (bind _returnvalue_2 (SaveGame|LoadGamefromSlot (Variables|Default|GetSaveSlotName)))
    (bind _assave_game_object (Utilities|Casting|CastToSaveGameObject _returnvalue_2))
    (Variables|Default|SetSaveGameData _assave_game_object)
    (else
      (bind _returnvalue_3 (SaveGame|CreateSaveGameObject "/Game/Blueprints/Saving/SaveGameObject.SaveGameObject_C"))
      (bind _output_get (Variables|Default|SetSaveGameData _returnvalue_3))
      (SaveGame|SaveGametoSlot _output_get (Variables|Default|GetSaveSlotName)))))

(fn SaveOptionsData
  (Utilities|Casting|CastToThirdPersonCharacter (Game|GetPlayerCharacter 0)))

(fn LoadOptionsData)