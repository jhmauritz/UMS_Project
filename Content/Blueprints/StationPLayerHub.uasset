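; StationPLayerHub holds pressed flags labeled by R and S number across five R groups and caches a reference to the ThirdPersonCharacter player.
; Tick polls every flag through a Sequence, and each true flag starts its own one-second Delay that clears it, turning presses into momentary signals.
; Nothing in these graphs sets or otherwise uses the flags.
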(event EventBeginPlay
  (bind _asthird_person_character (Utilities|Casting|CastToThirdPersonCharacter (Game|GetPlayerCharacter 0)))
  (Variables|Default|SetPlayerRef _asthird_person_character))

(event EventTick
  (params (DeltaSeconds :type Float%20%28single-precision%29))
  (Utilities|FlowControl|Sequence
    (:then_0
      (if (Variables|Default|GetR1_S1_Pressed)
        (Utilities|FlowControl|Delay 1.0)
        (Variables|Default|SetR1_S1_Pressed false)))
    (:then_1
      (if (Variables|Default|GetR1_S2_Pressed)
        (Utilities|FlowControl|Delay 1.0)
        (Variables|Default|SetR1_S2_Pressed false)))
    (:then_2
      (if (Variables|Default|GetR2_S1_Pressed)
        (Utilities|FlowControl|Delay 1.0)
        (Variables|Default|SetR2_S1_Pressed false)))
    (:then_3
      (if (Variables|Default|GetR2_S2_Pressed)
        (Utilities|FlowControl|Delay 1.0)
        (Variables|Default|SetR2_S2_Pressed false)))
    (:then_4
      (if (Variables|Default|GetR2_S3_Pressed)
        (Utilities|FlowControl|Delay 1.0)
        (Variables|Default|SetR2_S3_Pressed false)))
    (:then_5
      (if (Variables|Default|GetR3_S1_Pressed)
        (Utilities|FlowControl|Delay 1.0)
        (Variables|Default|SetR3_S1_Pressed false)))
    (:then_6
      (if (Variables|Default|GetR3_S2_Pressed)
        (Utilities|FlowControl|Delay 1.0)
        (Variables|Default|SetR3_S2_Pressed false)))
    (:then_7
      (if (Variables|Default|GetR3_S3_Pressed)
        (Utilities|FlowControl|Delay 1.0)
        (Variables|Default|SetR3_S3_Pressed false)))
    (:then_8
      (if (Variables|Default|GetR3_S4_Pressed)
        (Utilities|FlowControl|Delay 1.0)
        (Variables|Default|SetR3_S4_Pressed false)))
    (:then_9
      (if (Variables|Default|GetR4_S1_Pressed)
        (Utilities|FlowControl|Delay 1.0)
        (Variables|Default|SetR4_S1_Pressed false)))
    (:then_10
      (if (Variables|Default|GetR4_S2_Pressed)
        (Utilities|FlowControl|Delay 1.0)
        (Variables|Default|SetR4_S2_Pressed false)))
    (:then_11
      (if (Variables|Default|GetR4_S3_Pressed)
        (Utilities|FlowControl|Delay 1.0)
        (Variables|Default|SetR4_S3_Pressed false)))
    (:then_12
      (if (Variables|Default|GetR5_S1_Pressed)
        (Utilities|FlowControl|Delay 1.0)
        (Variables|Default|SetR5_S1_Pressed false)))
    (:then_13
      (if (Variables|Default|GetR5_S2_Pressed)
        (Utilities|FlowControl|Delay 1.0)
        (Variables|Default|SetR5_S2_Pressed false)))))

(fn ConstructionScript)