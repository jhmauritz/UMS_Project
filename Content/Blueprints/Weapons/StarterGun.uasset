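; Starter gun weapon Blueprint that removes itself when the player hub's LoadLevel actor begins teleporting.
; In the Player_HUB level, BeginPlay caches that actor and Tick polls its IsTeleporting flag to destroy the gun.
; Parent BeginPlay and Tick calls sit inside the level-name check, so the visible wiring runs them only in the hub.
; The Fire function is empty.
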(event EventBeginPlay
  (bind _returnvalue (Game|GetCurrentLevelName true))
  (if (Utilities|Enum|Equal(Enum) _returnvalue "Player_HUB")
    (bind _returnvalue_2 (Actor|GetActorOfClass "/Game/Blueprints/LoadLevel.LoadLevel_C"))
    (Variables|Default|SetNewVar_0 _returnvalue_2)
    (|CallParentFunction)))

(event Collision|EventActorBeginOverlap
  (params (OtherActor :type Actor%20Object%20Reference))
  (|CallParentFunction OtherActor) ; This node is disabled and will not be called.\nDrag off pins to build functionality.
)

(event EventTick
  (params (DeltaSeconds :type Float%20%28single-precision%29))
  (bind _returnvalue (Game|GetCurrentLevelName true))
  (if (Utilities|Enum|Equal(Enum) _returnvalue "Player_HUB")
    (if (Variables|/Game/Blueprints/LoadLevel.LoadLevel_C|GetIsTeleporting (Variables|Default|GetNewVar_0))
      (Actor|DestroyActor))
    (|CallParentFunction DeltaSeconds)))

(fn ConstructionScript
  (|CallParentFunction))

(fn Fire)