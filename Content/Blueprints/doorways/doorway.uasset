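; Doorway Blueprint for a door that the player opens and closes with the E key while near it.
; Overlap with a Box trigger enables input from player controller 0, and end overlap disables it, with no check on which actor overlaps.
; E toggles the DoorClosed flag and plays or reverses a timeline, which sets the pivot's yaw as an absolute world rotation.
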(event OnComponentEndOverlap(Box)
  (params (OverlappedComponent :type Primitive%20Component%20Object%20Reference) (OtherActor :type Actor%20Object%20Reference) (OtherComp :type Primitive%20Component%20Object%20Reference) (OtherBodyIndex :type Integer))
  ;[1 1 1] enable/disable input
  (Input|DisableInput (Game|GetPlayerController 0)))

(event OnComponentBeginOverlap(Box)
  (params (OverlappedComponent :type Primitive%20Component%20Object%20Reference) (OtherActor :type Actor%20Object%20Reference) (OtherComp :type Primitive%20Component%20Object%20Reference) (OtherBodyIndex :type Integer) (bFromSweep :type Boolean) (SweepResult :type Hit%20Result%20Structure%20%28by%20ref%29))
  ;[1 1 1] enable/disable input
  (Input|EnableInput (Game|GetPlayerController 0)))

(event Input|KeyboardEvents|E
  (params (Key :type Key%20Structure :default "None"))
  ;[1 1 1] open/close door
  (:Pressed
    (if (Variables|Default|Getdoor_closed)
      (Variables|Default|Setdoor_closed false)
      (bind _newtrack_0 (Timeline|open/close%20door Play)
        (:Update
          (Transformation|SetWorldRotation (Variables|Default|Getdoor%20pivot%20point) (Math|Rotator|MakeRotator 0.0 0.0 _newtrack_0) false false)))
      (else
        (Variables|Default|Setdoor_closed true)
        (Timeline|open/close%20door Reverse)))))

(fn ConstructionScript)